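; Trap_WaterUP is a trap that periodically sprays, launching and damaging any player caught in it.
; From BeginPlay it loops endlessly, using one shared delay to switch the particle system and the overlap volume's overlap events on and off together.
; A player beginning overlap is launched along the direction from the particle system to their location, scaled by LaunchVelocity, and takes Damage.
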(event `self.ReceiveBeginPlay`
  (bind _particlesystem (`self.ParticleSystem`))
  (`KismetSystemLibrary.Delay` (`self.DelayToSpray`) :!label _label)
  (`ActorComponent.Activate` _particlesystem false)
  (set `PrimitiveComponent.bGenerateOverlapEvents` true (`self.Overlap`))
  (`KismetSystemLibrary.Delay` (`self.DelayToSpray`))
  (`ActorComponent.Deactivate` _particlesystem)
  (set `PrimitiveComponent.bGenerateOverlapEvents` false (`self.Overlap`))
  (goto _label))

(event `self.Overlap.OnComponentBeginOverlap`
  (params (OverlappedComponent :type "PrimitiveComponent Object Reference") (OtherActor :type "Actor Object Reference") (OtherComp :type "PrimitiveComponent Object Reference") (OtherBodyIndex :type Integer) (bFromSweep :type Boolean) (SweepResult :type "HitResult Structure (by ref)"))
  (bind _asplayer (cast `/Game/GrandmotherVsZombies/Blueprints/Player/Player` OtherActor))
  (`Character.LaunchCharacter` _asplayer (* (`KismetMathLibrary.GetDirectionUnitVector` (`SceneComponent.K2_GetComponentLocation` (`self.ParticleSystem`)) (`self.K2_GetActorLocation` _asplayer)) (`self.Launch Velocity`)) false false)
  (`GameplayStatics.ApplyDamage` _asplayer (`self.Damage`)))

(fn `UserConstructionScript`)