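; Weapon pickup actor that shows a name and image prompt when the player is near and can be picked up with Interact.
; Sphere overlaps toggle the widget and a CanPick flag, which gates the call to the player's PickupItem.
; ClearAll destroys the sphere and hides the prompt to end pickup behaviour.
; The construction script stamps the actor's own class into its WeaponInfo struct, which holds the weapon's stats and assets.
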(event `self.Sphere.OnComponentBeginOverlap`
  (params (OverlappedComponent :type "PrimitiveComponent Object Reference") (OtherActor :type "Actor Object Reference") (OtherComp :type "PrimitiveComponent Object Reference") (OtherBodyIndex :type Integer) (bFromSweep :type Boolean) (SweepResult :type "HitResult Structure (by ref)"))
  (bind ((`Image_35_FC8E9AED475132FDF93D2A95AEA77B00` _image) (`Name_18_2F685C70471C4E5C676675BA20A74336` _name)) (break `/Game/GrandmotherVsZombies/Blueprints/Weapons/WeaponInfo` (`self.WeaponInfo`)))
  (bind _aspickup_wb (cast `/Game/GrandmotherVsZombies/Blueprints/GameUI/PickupUI/PickupWB` (`WidgetComponent.GetUserWidgetObject` (`self.Widget`)) :!pure true))
  (bind _asplayer (cast `/Game/GrandmotherVsZombies/Blueprints/Player/Player` OtherActor))
  (set `self.PlayerRef` _asplayer)
  (`SceneComponent.SetVisibility` (`self.Widget`) true false)
  (set `self.CanPick?` true)
  (`self.EnableInput` (`GameplayStatics.GetPlayerController` 0))
  (set `/Game/GrandmotherVsZombies/Blueprints/GameUI/PickupUI/PickupWB.ItemInfo` (`KismetTextLibrary.Conv_StringToText` (`KismetStringLibrary.Concat_StrStr` _name " [ F ]")) _aspickup_wb)
  (set `/Game/GrandmotherVsZombies/Blueprints/GameUI/PickupUI/PickupWB.ItemImage` _image _aspickup_wb))

(event `self.Sphere.OnComponentEndOverlap`
  (params (OverlappedComponent :type "PrimitiveComponent Object Reference") (OtherActor :type "Actor Object Reference") (OtherComp :type "PrimitiveComponent Object Reference") (OtherBodyIndex :type Integer))
  (bind _asplayer (cast `/Game/GrandmotherVsZombies/Blueprints/Player/Player` OtherActor))
  (set `self.PlayerRef` _asplayer)
  (`SceneComponent.SetVisibility` (`self.Widget`) false false)
  (set `self.CanPick?` false))

(event `InputAction|Interact`
  (params (Key :type "Key Structure"))
  (:`Pressed`
    (if (`self.CanPick?`)
      (`/Game/GrandmotherVsZombies/Blueprints/Player/Player.PickupItem` (`self.PlayerRef`) self))))

(event `ClearAll`
  (`ActorComponent.K2_DestroyComponent` (`self.Sphere`))
  (`SceneComponent.SetVisibility` (`self.Widget`) false false)
  (set `self.CanPick?` false))

(fn `UserConstructionScript`
  (bind (_weaponinfo_weapontype _weaponinfo_image _weaponinfo_class _weaponinfo_name _weaponinfo_equipsocket _weaponinfo_unequipsocket _weaponinfo_damage _weaponinfo_firerate _weaponinfo_range _weaponinfo_clipsize _weaponinfo_currentammo _weaponinfo_maxammo _weaponinfo_pickupammo _weaponinfo_firesound _weaponinfo_firemontage _weaponinfo_reloademontage) (break `/Game/GrandmotherVsZombies/Blueprints/Weapons/WeaponInfo` (`self.WeaponInfo`)))
  (set `self.WeaponInfo` (make `/Game/GrandmotherVsZombies/Blueprints/Weapons/WeaponInfo` _weaponinfo_weapontype _weaponinfo_image (`GameplayStatics.GetObjectClass` self) _weaponinfo_name _weaponinfo_equipsocket _weaponinfo_unequipsocket _weaponinfo_damage _weaponinfo_firerate _weaponinfo_range _weaponinfo_clipsize _weaponinfo_currentammo _weaponinfo_maxammo _weaponinfo_pickupammo _weaponinfo_firesound _weaponinfo_firemontage _weaponinfo_reloademontage)))