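; ZombieAI_01 is a zombie character Blueprint that takes damage from bullets and dies when its health runs out.
; On actor overlap with a Bullet, it subtracts a fixed amount of Health and destroys itself at zero or below.
; UpdateWalkSpeed sets the CharacterMovement max walk speed to a given value, and nothing in this file calls it.
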(event `self.ReceiveActorBeginOverlap`
  (params (OtherActor :type "Actor Object Reference"))
  (cast `/Game/GrandmotherVsZombies/Blueprints/Bullet` OtherActor)
  (set `self.Health` (- (`self.Health`) 15.0))
  (if (<= (`self.Health`) 0.0)
    (`self.K2_DestroyActor`)))

(fn `Update Walk Speed`
  (params (NewWalkSpeed :type "Float (double-precision)"))
  (set `CharacterMovementComponent.MaxWalkSpeed` NewWalkSpeed (`self.CharacterMovement`)))

(fn `UserConstructionScript`)