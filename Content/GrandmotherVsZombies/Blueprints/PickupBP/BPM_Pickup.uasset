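; Base pickup actor that the player collects with the Interact input while in range.
; A sphere overlap with the Player sets CanPickup, enables input and shows a PickupWB widget with the item's name, key hint and image; leaving hides it.
; Interact, gated by CanPickup, passes the actor to the Player's ItemPickup.
; The construction script stamps the actor's own class into PickupInfo, keeping its other fields.
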(event `self.Sphere.OnComponentBeginOverlap`
  (params (OverlappedComponent :type "PrimitiveComponent Object Reference") (OtherActor :type "Actor Object Reference") (OtherComp :type "PrimitiveComponent Object Reference") (OtherBodyIndex :type Integer) (bFromSweep :type Boolean) (SweepResult :type "HitResult Structure (by ref)"))
  (bind ((`Name_2_26CC25284FE43DA31F7CE7963283CDB5` _name) (`Image_8_2F5CF5B2414F9036398610B335745F2C` _image)) (break `/Game/GrandmotherVsZombies/Blueprints/PickupBP/S_PickupInfo` (`self.PickupInfo`)))
  (bind _aspickup_wb (cast `/Game/GrandmotherVsZombies/Blueprints/GameUI/PickupUI/PickupWB` (`WidgetComponent.GetUserWidgetObject` (`self.Widget`)) :!pure true))
  (cast `/Game/GrandmotherVsZombies/Blueprints/Player/Player` OtherActor)
  (set `self.CanPickup?` true)
  (`SceneComponent.SetVisibility` (`self.Widget`) true false)
  (`self.EnableInput` (`GameplayStatics.GetPlayerController` 0))
  (set `/Game/GrandmotherVsZombies/Blueprints/GameUI/PickupUI/PickupWB.ItemInfo` (`KismetTextLibrary.Conv_StringToText` (`KismetStringLibrary.Concat_StrStr` (`KismetTextLibrary.Conv_TextToString` _name) " [ F ]")) _aspickup_wb)
  (set `/Game/GrandmotherVsZombies/Blueprints/GameUI/PickupUI/PickupWB.ItemImage` _image _aspickup_wb))

(event `self.Sphere.OnComponentEndOverlap`
  (params (OverlappedComponent :type "PrimitiveComponent Object Reference") (OtherActor :type "Actor Object Reference") (OtherComp :type "PrimitiveComponent Object Reference") (OtherBodyIndex :type Integer))
  (cast `/Game/GrandmotherVsZombies/Blueprints/Player/Player` OtherActor)
  (set `self.CanPickup?` false)
  (`SceneComponent.SetVisibility` (`self.Widget`) false false))

(event `InputAction|Interact`
  (params (Key :type "Key Structure"))
  (:`Pressed`
    (if (`self.CanPickup?`)
      (`/Game/GrandmotherVsZombies/Blueprints/Player/Player.ItemPickup` (cast `/Game/GrandmotherVsZombies/Blueprints/Player/Player` (`GameplayStatics.GetPlayerCharacter` 0) :!pure true) self))))

(fn `UserConstructionScript`
  (bind (_pickupinfo_class _pickupinfo_name _pickupinfo_amount _pickupinfo_image) (break `/Game/GrandmotherVsZombies/Blueprints/PickupBP/S_PickupInfo` (`self.PickupInfo`)))
  (set `self.PickupInfo` (make `/Game/GrandmotherVsZombies/Blueprints/PickupBP/S_PickupInfo` (`GameplayStatics.GetObjectClass` self) _pickupinfo_name _pickupinfo_amount _pickupinfo_image)))